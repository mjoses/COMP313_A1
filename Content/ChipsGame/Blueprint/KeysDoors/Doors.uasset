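; Locked door actor that destroys itself with a sound when a character holding the matching key type overlaps it.
; On overlap it shows an inspect prompt, then checks the MyCharacter's OwnedKeys against RequiredKeyType.
; Interact toggles a dialogue widget showing the door's text, and the character leaving the overlap removes both widgets.
; An OpenLevelByName node is left unconnected, so no level loads.
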(event OnComponentBeginOverlap(Overlap)
  (params (OverlappedComponent :type Primitive%20Component%20Object%20Reference) (OtherActor :type Actor%20Object%20Reference) (OtherComp :type Primitive%20Component%20Object%20Reference) (OtherBodyIndex :type Integer) (bFromSweep :type Boolean) (SweepResult :type Hit%20Result%20Structure%20%28by%20ref%29))
  (Utilities|FlowControl|Sequence
    (:then_0
      (bind _returnvalue (UserInterface|CreateWidget "/Game/ChipsGame/Widgets/InspectionD.InspectionD_C" (Game|GetPlayerController 0)))
      (bind _output_get (Variables|Default|SetInspectD _returnvalue))
      (UserInterface|Viewport|AddtoViewport _output_get 0)
      (Variables|/Game/ChipsGame/Widgets/InspectionD.InspectionD_C|SetInspectText (Variables|Default|GetInspectD) "Press \"E\" to inspect!"))
    (:then_1
      (bind _asmy_character (Utilities|Casting|CastToMyCharacter OtherActor))
      (for _array_element (Variables|/Game/ChipsGame/Blueprint/Characters/MyCharacter.MyCharacter_C|GetOwnedKeys _asmy_character)
        (if (Utilities|Enum|Equal(Enum) _array_element (Variables|Default|GetRequiredKeyType))
          (Utilities|Casting|CastTomyGameInstance (Game|GetGameInstance))
          (Audio|PlaySound2D "/Game/ChipsGame/Audio/DoorSound.DoorSound" 1.0 1.0 0.0 0 0)
          (Actor|DestroyActor))))))

(event OnComponentEndOverlap(Overlap)
  (params (OverlappedComponent :type Primitive%20Component%20Object%20Reference) (OtherActor :type Actor%20Object%20Reference) (OtherComp :type Primitive%20Component%20Object%20Reference) (OtherBodyIndex :type Integer))
  (Utilities|Casting|CastToMyCharacter OtherActor)
  (Utilities|FlowControl|Sequence
    (:then_0
      (Utilities|IsValid (Variables|Default|GetDialogue_Wid)
        (:Is%20Valid
          (Widget|RemovefromParent (Variables|Default|GetDialogue_Wid))
          (Variables|Default|SetDialogue_Wid 0))))
    (:then_1
      (Utilities|IsValid (Variables|Default|GetInspectD)
        (:Is%20Valid
          (Widget|RemovefromParent (Variables|Default|GetInspectD))
          (Variables|Default|SetInspectD 0))))))

(event EventInteract
  (Utilities|IsValid (Variables|Default|GetDialogue_Wid)
    (:Is%20Valid
      (Widget|RemovefromParent (Variables|Default|GetDialogue_Wid))
      (Variables|Default|SetDialogue_Wid 0))
    (:Is%20Not%20Valid
      (bind _returnvalue (UserInterface|CreateWidget "/Game/ChipsGame/Widgets/Dialogue_Wid.Dialogue_Wid_C" (Game|GetPlayerController 0)))
      (bind _output_get (Variables|Default|SetDialogue_Wid _returnvalue))
      (UserInterface|Viewport|AddtoViewport _output_get 0)
      (Variables|/Game/ChipsGame/Widgets/Dialogue_Wid.Dialogue_Wid_C|SetDialogue%20Text (Variables|Default|GetDialogue_Wid) (Variables|Default|GetMyText)))))

(fn ConstructionScript)