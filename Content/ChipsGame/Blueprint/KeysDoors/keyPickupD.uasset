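; Pickup actor for key D that plays a sound and shows a timed message when first overlapped.
; A DoOnce gate plays the sound on the first overlap by any actor, then casts it to MyCharacter.
; On success it displays an InspectionD widget with the key text, waits three seconds, then removes the widget and destroys itself.
; The graph does not record the key on the character.
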(event OnComponentBeginOverlap(Overlap)
  (params (OverlappedComponent :type Primitive%20Component%20Object%20Reference) (OtherActor :type Actor%20Object%20Reference) (OtherComp :type Primitive%20Component%20Object%20Reference) (OtherBodyIndex :type Integer) (bFromSweep :type Boolean) (SweepResult :type Hit%20Result%20Structure%20%28by%20ref%29))
  (Utilities|FlowControl|DoOnce false
    (:Completed
      (Audio|PlaySound2D "/Game/ChipsGame/Audio/KeyPickSound.KeyPickSound" 1.0 1.0 0.0 0 0)
      (Utilities|Casting|CastToMyCharacter OtherActor)
      (bind _returnvalue (UserInterface|CreateWidget "/Game/ChipsGame/Widgets/InspectionD.InspectionD_C"))
      (bind _output_get (Variables|Default|SetKeyT _returnvalue))
      (UserInterface|Viewport|AddtoViewport _output_get 0)
      (Variables|/Game/ChipsGame/Widgets/InspectionD.InspectionD_C|SetInspectText (Variables|Default|GetKeyT) (Variables|Default|GetKeyText))
      (Utilities|FlowControl|Delay 3.0)
      (Utilities|IsValid (Variables|Default|GetKeyT)
        (:Is%20Valid
          (Widget|RemovefromParent (Variables|Default|GetKeyT))
          (Variables|Default|SetKeyT 0)
          (Actor|DestroyActor))))))

(fn ConstructionScript)