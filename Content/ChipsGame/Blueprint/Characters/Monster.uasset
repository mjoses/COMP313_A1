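; Monster character that chases a seen MyCharacter and kills it on reaching it.
; PawnSensing plays the monster audio on the first sighting only and starts AIMoveTo toward the player; success plays a death animation on player 0 and sets IsDead.
; A failed chase starts a delayed patrol loop between Target1 and Target2.
; It also carries control-yaw-relative movement axis input, gated by DisableMovement.
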(event OnSeePawn(PawnSensing)
  (params (Pawn :type Pawn%20Object%20Reference))
  ;[1 1 1] AI
  (Utilities|FlowControl|Sequence
    (:then_0
      (Utilities|FlowControl|DoOnce false
        (:Completed
          (Audio|Components|Audio|Play (Variables|Default|GetMonsterAudio) 0.0))))
    (:then_1
      (bind _asmy_character (Utilities|Casting|CastToMyCharacter Pawn))
      (AI|AIMoveTo self "0, 0, 0" _asmy_character 5.0 false
        (:OnSuccess
          (Components|Animation|PlayAnimation (Variables|/Script/Engine.Character|GetMesh (Game|GetPlayerCharacter 0)) "/Game/AnimStarterPack/Death_1.Death_1" false)
          (Variables|/Game/ChipsGame/Blueprint/Characters/MyCharacter.MyCharacter_C|SetisDead _asmy_character true))
        (:OnFail
          (Utilities|FlowControl|Delay 3.0 :!label _label)
          (AI|AIMoveTo self "0, 0, 0" (Variables|Default|GetTarget1) 5.0 false
            (:OnSuccess
              (Utilities|FlowControl|Delay 3.0)
              (AI|AIMoveTo self "0, 0, 0" (Variables|Default|GetTarget2) 5.0 false
                (:OnSuccess
                  (goto _label))))))))))

(event Input|AxisEvents|InputAxisMoveRight
  (params (AxisValue :type Float%20%28single-precision%29))
  ;[1 1 1] Movements
  (if (not (Variables|Default|GetDisableMovement))
    (Pawn|Input|AddMovementInput (Math|Vector|GetRightVector (Math|Rotator|MakeRotator 0.0 0.0 (.Yaw (Math|Rotator|BreakRotator (Pawn|GetControlRotation :!class /Script/Engine.Pawn))))) AxisValue false)))

(event Input|AxisEvents|InputAxisMoveForward
  (params (AxisValue :type Float%20%28single-precision%29))
  ;[1 1 1] Movements
  (if (not (Variables|Default|GetDisableMovement))
    (Pawn|Input|AddMovementInput (Math|Vector|GetForwardVector (Math|Rotator|MakeRotator 0.0 0.0 (.Yaw (Math|Rotator|BreakRotator (Pawn|GetControlRotation :!class /Script/Engine.Pawn))))) AxisValue false)))

(fn ConstructionScript)