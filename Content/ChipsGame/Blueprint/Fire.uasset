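; Fire hazard actor that kills the player character on contact with its box.
; On overlap, it disables the character's input, plays a non-looping prone death animation, and DiedFunction sets IsDead on player 0's character.
; Tick calls Play on the Fire component from time zero every frame.
; A delayed destroy of the character exists but is not connected, so it never runs.
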(event OnComponentBeginOverlap(Box)
  (params (OverlappedComponent :type Primitive%20Component%20Object%20Reference) (OtherActor :type Actor%20Object%20Reference) (OtherComp :type Primitive%20Component%20Object%20Reference) (OtherBodyIndex :type Integer) (bFromSweep :type Boolean) (SweepResult :type Hit%20Result%20Structure%20%28by%20ref%29))
  (bind _asmy_character (Utilities|Casting|CastToMyCharacter OtherActor))
  (Input|DisableInput _asmy_character 0)
  (Components|Animation|PlayAnimation (Variables|/Script/Engine.Character|GetMesh _asmy_character) "/Game/AnimStarterPack/Prone_Death_1.Prone_Death_1" false)
  (CallFunction|DiedFunction))

(event EventTick
  (params (DeltaSeconds :type Float%20%28single-precision%29))
  (Audio|Components|Audio|Play (Variables|Default|Getfire) 0.0))

(fn ConstructionScript)

(fn DiedFunction
  (bind _asmy_character (Utilities|Casting|CastToMyCharacter (Game|GetPlayerCharacter 0)))
  (Variables|/Game/ChipsGame/Blueprint/Characters/MyCharacter.MyCharacter_C|SetisDead _asmy_character true))